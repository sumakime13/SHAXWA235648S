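; Inventory component that stores items in a fixed-size array of slots and shows them in an Inventory widget.
; BeginPlay sizes the array and caches the player's CharacterMaster, which ToggleInventory passes to a newly created widget with an opening animation.
; AddToInventory tops up matching partial stacks, recursing with any overflow, or writes to the first empty slot, and always returns true.
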(event EventBeginPlay
  (CallFunction|PrepareInventory)
  (bind _ascharacter_master (Utilities|Casting|CastToCharacterMaster (Game|GetPlayerCharacter 0)))
  (Variables|Default|Setplayer _ascharacter_master))

(event EventTick
  (params (DeltaSeconds :type Float%20%28single-precision%29)))

(fn ToggleInventory
  (bind _returnvalue (UserInterface|CreateWidget "/Game/Data/Widget/inventory/inventory.inventory_C" 0 self (Variables|Default|Getplayer)))
  (bind _output_get (Variables|Default|SetInventoryWidget _returnvalue))
  (UserInterface|Viewport|AddtoViewport _output_get 0)
  (UserInterface|Animation|PlayAnimation _returnvalue (Variables|/Game/Data/Widget/inventory/inventory.inventory_C|GetOpen/Close _returnvalue) 0.0 1 "Forward" 1.0))

(fn AddtoInventory
  (params (ContentToAdd :type Slot%20Struct%20Structure))
  (if (.isstackable (.itemstruct ContentToAdd))
    (bind _stackindex (Utilities|HasPartialStack ContentToAdd)
      (:true
        (CallFunction|AddtoStack ContentToAdd _stackindex))
      (:false
        (CallFunction|CreateStack ContentToAdd :!label _label)))
    (else
      (goto _label)))
  (return true))

(fn PrepareInventory
  (Utilities|Array|Resize (Variables|Default|GetInventory) (Variables|Default|GetNumberOfSlots)))

(fn CreateStack
  (params (ContentToAdd :type Slot%20Struct%20Structure))
  (bind _inventory (Variables|Default|GetInventory))
  (Utilities|Array|SetArrayElem _inventory (Utilities|Array|FindItem _inventory (Utilities|Struct|MakeSlotStruct "(Name_item_17_5A41B4394055FBF8273386BD197B73B3=\"\",IsStackable_20_A16B51084D2DF62B08328EB1B5975190=False,Image_2_7DDD76AD4F5AADF977962CA053B6C706=None,Description_11_266DEAFA4030B0DCA39B9589CE496BD2=\"\",isConsumable_21_CDA92D334F99027C45336C9966D3E754=False,MaxStackSize_22_56E9A12144B879DDD30978B88AD0BDDA=0,Durabiity_29_567C23A9472251F503DC9994EC4B701E=0.000000,Enum_8_8EC0CA22443C580A827C78A54E275434=NewEnumerator0,Class_28_14F69CAD46A9C60701D962A466652AE9=None,Buy_33_D59CAA544B1949152BA451A620A79F52=0,Sell_35_41D5606F4E724C1C3C51DDB38B3E58E9=0,Sell?_37_7AD756C64F157AC4661CBA8F8BFD209C=False)")) ContentToAdd))

(fn AddtoStack
  (params (SlotStruncture :type Slot%20Struct%20Structure) (SlotIndex :type Integer))
  (bind _inventory (Variables|Default|GetInventory))
  (bind _inventory_2 (Variables|Default|GetInventory))
  (bind _maxstacksize (Utilities|Struct|BreakItemDefinedStruct (.itemstruct SlotStruncture)))
  (bind _output (Utilities|Array|Get(acopy) _inventory SlotIndex))
  (bind _output_2 (Utilities|Array|Get(acopy) _inventory_2 SlotIndex))
  (bind _output_get (LocalVariables|SetCurrentQuantity (.quanlity _output)))
  (if (> (+ _output_get (.Quanlity (Utilities|Struct|BreakSlotStruct SlotStruncture))) (.maxstacksize (.itemstruct _output)))
    (Utilities|Array|SetArrayElem (Variables|Default|GetInventory) SlotIndex (Utilities|Struct|MakeSlotStruct (.itemstruct SlotStruncture) _maxstacksize))
    (CallFunction|AddtoInventory (Utilities|Struct|MakeSlotStruct (.itemstruct SlotStruncture) (- (.quanlity SlotStruncture) (- _maxstacksize (LocalVariables|GetCurrentQuantity)))))
    (else
      (Utilities|Array|SetArrayElem _inventory_2 SlotIndex (Utilities|Struct|MakeSlotStruct (.itemstruct _output_2) (+ (.quanlity _output_2) (.quanlity SlotStruncture))))))
  (return))