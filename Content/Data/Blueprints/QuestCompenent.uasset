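; Quest component that keeps a slot-based quest log and opens the MyQuest widget to display it.
; On BeginPlay it sizes the Quest array to NumberOfSlots.
; AddtoMyQuest searches for a matching quest with a macro, then either overwrites that slot or writes into the first empty-struct slot.
; The overwrite path calls AddtoMyQuest again with the same quest, so a match recurses without a visible exit.
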(event EventBeginPlay
  (CallFunction|PrepareQuest))

(event EventTick
  (params (DeltaSeconds :type Float%20%28single-precision%29)))

(fn OpenMyQuest
  (bind _returnvalue (UserInterface|CreateWidget "/Game/Data/Blueprints/MyQuest.MyQuest_C" 0 self))
  (bind _output_get (Variables|Default|SetMyQuest _returnvalue))
  (UserInterface|Viewport|AddtoViewport _output_get 0))

(fn CreatetoStack
  (params (Quest%20Struct :type Quest%20Struct%20Structure))
  (bind _quest (Variables|Default|GetQuest))
  (Utilities|Array|SetArrayElem _quest (Utilities|Array|FindItem _quest (Utilities|Struct|MakeQuestStruct :Item (Utilities|Array|MakeArray ""))) Quest%20Struct))

(fn AddtoMyQuest
  (params (Quest%20Struct :type Quest%20Struct%20Structure))
  (bind _variable (Utilities|NewMacro0 Quest%20Struct)
    (:true
      (CallFunction|AddtoStack Quest%20Struct _variable))
    (:false
      (CallFunction|CreatetoStack Quest%20Struct)))
  (return))

(fn AddtoStack
  (params (Quest :type Quest%20Struct%20Structure) (Slot%20int :type Integer))
  (if true
    (Utilities|Array|SetArrayElem (Variables|Default|GetQuest) Slot%20int Quest)
    (CallFunction|AddtoMyQuest Quest)
    (return)))

(fn PrepareQuest
  (Utilities|Array|Resize (Variables|Default|GetQuest) (Variables|Default|GetNumberOfSlots)))