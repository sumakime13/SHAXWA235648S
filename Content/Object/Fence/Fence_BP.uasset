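; Fence Blueprint that builds a straight row of repeated meshes from its component's position toward a Target point, with no runtime logic.
; The construction script assigns MeshToSpawn to a Hierarchical Instanced Static Mesh and yaws it toward Target, ignoring height.
; It then clears and re-adds instances along local X, spaced by the component's local bounds Max X, with the count derived from the distance to Target.
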(event EventBeginPlay)

(event Collision|EventActorBeginOverlap
  (params (OtherActor :type Actor%20Object%20Reference)))

(event EventTick
  (params (DeltaSeconds :type Float%20%28single-precision%29)))

(fn ConstructionScript
  (bind _hierarchicalinstancedstaticmesh (Variables|Default|GetHierarchicalInstancedStaticMesh))
  (bind _hierarchicalinstancedstaticmesh_2 (Variables|Default|GetHierarchicalInstancedStaticMesh))
  (bind _hierarchicalinstancedstaticmesh_3 (Variables|Default|GetHierarchicalInstancedStaticMesh))
  (bind _target (Variables|Default|GetTarget))
  (bind (_x _y) (Math|Vector|BreakVector _target))
  (bind _relativelocation (Variables|/Script/Engine.SceneComponent|GetRelativeLocation _hierarchicalinstancedstaticmesh))
  (Components|StaticMesh|SetStaticMesh (Variables|Default|GetHierarchicalInstancedStaticMesh) (Variables|Default|GetMeshToSpawn))
  (Transformation|SetRelativeRotation (Variables|Default|GetHierarchicalInstancedStaticMesh) (Math|Rotator|FindLookatRotation _relativelocation (Math|Vector|MakeVector _x _y (.Z (Math|Vector|BreakVector _relativelocation)))) false false)
  (Utilities|FlowControl|Sequence
    (:then_0
      (Components|InstancedStaticMesh|ClearInstances _hierarchicalinstancedstaticmesh_3)
      (Components|InstancedStaticMesh|AddInstance _hierarchicalinstancedstaticmesh_3 (Math|Transform|MakeTransform "0.000000, 0,0.000000")))
    (:then_1
      (LocalVariables|SetDistance (Math|Vector|VectorLength (- (Variables|Default|GetTarget) (Variables|/Script/Engine.SceneComponent|GetRelativeLocation (Variables|Default|GetHierarchicalInstancedStaticMesh))))))
    (:then_2
      (for _index (range 0 (Math|Float|Floor (/ (LocalVariables|GetDistance) (.X (Math|Vector|BreakVector (.Max (Components|StaticMesh|GetLocalBounds (Variables|Default|GetHierarchicalInstancedStaticMesh))))))))
        (Components|InstancedStaticMesh|AddInstance _hierarchicalinstancedstaticmesh_2 (Math|Transform|MakeTransform (Math|Vector|MakeVector (* _index (.X (Math|Vector|BreakVector (.Max (Components|StaticMesh|GetLocalBounds _hierarchicalinstancedstaticmesh_2))))) 0.0 0.0) "0, 0,0.000000"))))))